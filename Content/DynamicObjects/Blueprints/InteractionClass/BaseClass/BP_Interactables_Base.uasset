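; Base interactable actor that, by interact type, toggles a hit component open or closed, destroys itself on collect, or calls an empty inspect stub.
; InteractItem flips the component's "Closed" tag and plays a timeline forward or in reverse on Stationary or Movable components.
; UpdateTransform builds the timeline's lerp endpoints from InteractDetails, masking optional location and rotation changes by LocationAxis and forcing unit scale.
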(event `/Game/DynamicObjects/Blueprints/InteractionClass/BaseClass/Interface/BP_InteractionInteraface.InteractRequest`
  (params (HitObject :type "PrimitiveComponent Object Reference"))
  ;[1 1 1] Interact request
  ;;[1 1 1] Ref hit object
  (set `self.HitObject` HitObject)
  ;;[1 1 1] Trigger based on interact type
  (switch `/Game/DynamicObjects/Blueprints/InteractionClass/BaseClass/ClassDefaults/E_InteractTypes` (`.InteractType_9_6D13FBF44DF31A9F60E3698C7E430CE7` (break `/Game/DynamicObjects/Blueprints/InteractionClass/BaseClass/ClassDefaults/ST_Interactable_Details` (`self.InteractDetails`)))
    (:`NewEnumerator1`
      ;;;[1 1 1] Trigger movement only on movable meshes
      (switch `EComponentMobility` (`SceneComponent.Mobility` (`self.HitObject`))
        (:`Stationary`
          _)
        (:`Movable`
          _))
      (if (not (`TimelineComponent.IsPlaying` (`self.Interact_TL`)))
        (`self.InteractItem`)))
    (:`NewEnumerator3`
      (`self.InspectItem`))
    (:`NewEnumerator4`
      (`self.CollectItem`))))

(fn `CollectItem`
  (`self.K2_DestroyActor`))

(fn `InspectItem`)

(fn `InteractItem`
  ;[1 1 1] Set animation play rate
  (`TimelineComponent.SetPlayRate` (`self.Interact_TL`) (`.AnimationPlayRate_15_0BBC4B1C40B1073AF15E82BB8BC34BB3` (break `/Game/DynamicObjects/Blueprints/InteractionClass/BaseClass/ClassDefaults/ST_Interactable_Details` (`self.InteractDetails`))))
  ;[1 1 1] Update transform
  (set `self.TransformA` (`self.UpdateTransform` true))
  (set `self.TransformB` (`self.UpdateTransform` false))
  ;[1 1 1] Check if item is closed/open and act accordingly
  (if (`ActorComponent.ComponentHasTag` (`self.HitObject`) "Closed")
    (`KismetArrayLibrary.Array_RemoveItem` (`ActorComponent.ComponentTags` (`self.HitObject`)) "Closed")
    ;[1 1 1] Play animation direction
    (`TimelineComponent.PlayFromStart` (`self.Interact_TL`))
    (else
      (`KismetArrayLibrary.Array_AddUnique` (`ActorComponent.ComponentTags` (`self.HitObject`)) "Closed")
      (`TimelineComponent.ReverseFromEnd` (`self.Interact_TL`)))))

(fn `UpdateTransform`
  (params (`Start?` :type Boolean))
  (returns (ReturnValue :type "Transform Structure"))
  (bind ((`ItemName_29_F946D14143B55A5AEFB43D98A027DBC4` _itemname) (`ItemDetail_27_7CB59E7A46F11E36ED4C7595FCD737FC` _itemdetail) (`ItemImage_32_74EAD52642E83FDDC309F2A87E74CA5A` _itemimage) (`StartTransform_7_FED52DEE4DFCB9106AF6B893014A0A75` _starttransform) (`EndTransform_8_4077500841C363CE3AC7E5B28933C1B4` _endtransform)) (break `/Game/DynamicObjects/Blueprints/InteractionClass/BaseClass/ClassDefaults/ST_Interactable_Details` (`self.InteractDetails`)))
  (bind ((`ItemName_29_F946D14143B55A5AEFB43D98A027DBC4` _itemname_2) (`ItemDetail_27_7CB59E7A46F11E36ED4C7595FCD737FC` _itemdetail_2) (`ItemImage_32_74EAD52642E83FDDC309F2A87E74CA5A` _itemimage_2) (`StartTransform_7_FED52DEE4DFCB9106AF6B893014A0A75` _starttransform_2) (`EndTransform_8_4077500841C363CE3AC7E5B28933C1B4` _endtransform_2)) (break `/Game/DynamicObjects/Blueprints/InteractionClass/BaseClass/ClassDefaults/ST_Interactable_Details` (`self.InteractDetails`)))
  (bind (_relativerotation_roll _relativerotation_pitch _relativerotation_yaw) (`KismetMathLibrary.BreakRotator` (`SceneComponent.RelativeRotation` (`self.HitObject`))))
  (bind (_relativelocation_x _relativelocation_y _relativelocation_z) (`KismetMathLibrary.BreakVector` (`SceneComponent.RelativeLocation` (`self.HitObject`))))
  (bind _x (.x (.location (`KismetMathLibrary.SelectTransform` _starttransform_2 _endtransform_2 (`local.Start?`)))))
  (bind _y (.y (.location (`KismetMathLibrary.SelectTransform` _starttransform_2 _endtransform_2 (`local.Start?`)))))
  (bind _z (.z (.location (`KismetMathLibrary.SelectTransform` _starttransform_2 _endtransform_2 (`local.Start?`)))))
  (bind _roll (.roll (.rotation (`KismetMathLibrary.SelectTransform` _starttransform _endtransform (`local.Start?`)))))
  (bind _pitch (.pitch (.rotation (`KismetMathLibrary.SelectTransform` _starttransform _endtransform (`local.Start?`)))))
  (bind _yaw (.yaw (.rotation (`KismetMathLibrary.SelectTransform` _starttransform _endtransform (`local.Start?`)))))
  ;[1 1 1] Returning transform
  (return (`KismetMathLibrary.MakeTransform` (`KismetMathLibrary.SelectVector` (select `/Game/DynamicObjects/Blueprints/InteractionClass/BaseClass/ClassDefaults/E_MoveAxis` (`.LocationAxis_18_8577B3A04EB5677CCAACAF8B7381A5AF` (break `/Game/DynamicObjects/Blueprints/InteractionClass/BaseClass/ClassDefaults/ST_Interactable_Details` (`self.InteractDetails`))) :`NewEnumerator0` (`KismetMathLibrary.MakeVector` _x _relativelocation_y _relativelocation_z) :`NewEnumerator1` (`KismetMathLibrary.MakeVector` _relativelocation_x _y _relativelocation_z) :`NewEnumerator2` (`KismetMathLibrary.MakeVector` _relativelocation_x _relativelocation_y _z) :`NewEnumerator3` (`KismetMathLibrary.MakeVector` _x _y _relativelocation_z) :`NewEnumerator4` (`KismetMathLibrary.MakeVector` _x _relativelocation_y _z) :`NewEnumerator5` (`KismetMathLibrary.MakeVector` _relativelocation_x _y _z) :`NewEnumerator6` (`KismetMathLibrary.MakeVector` _x _y _z)) (`SceneComponent.RelativeLocation` (`self.HitObject`)) (`.InflictLocationChange?_24_BE5920A84FFC3B0E57C584BF3A8ADAE0` (break `/Game/DynamicObjects/Blueprints/InteractionClass/BaseClass/ClassDefaults/ST_Interactable_Details` (`self.InteractDetails`)))) (`KismetMathLibrary.SelectRotator` (`SceneComponent.RelativeRotation` (`self.HitObject`)) (select `/Game/DynamicObjects/Blueprints/InteractionClass/BaseClass/ClassDefaults/E_MoveAxis` (`.LocationAxis_18_8577B3A04EB5677CCAACAF8B7381A5AF` (break `/Game/DynamicObjects/Blueprints/InteractionClass/BaseClass/ClassDefaults/ST_Interactable_Details` (`self.InteractDetails`))) :`NewEnumerator0` (`KismetMathLibrary.MakeRotator` _roll _relativerotation_pitch _relativerotation_yaw) :`NewEnumerator1` (`KismetMathLibrary.MakeRotator` _relativerotation_roll _pitch _relativerotation_yaw) :`NewEnumerator2` (`KismetMathLibrary.MakeRotator` _relativerotation_roll _relativerotation_pitch _yaw) :`NewEnumerator3` (`KismetMathLibrary.MakeRotator` _roll _pitch _relativerotation_yaw) :`NewEnumerator4` (`KismetMathLibrary.MakeRotator` _roll _relativerotation_pitch _yaw) :`NewEnumerator5` (`KismetMathLibrary.MakeRotator` _relativerotation_roll _pitch _yaw) :`NewEnumerator6` (`KismetMathLibrary.MakeRotator` _roll _pitch _yaw)) (not (`.InflictRotationChange?_22_DBB1F1714ECF4B8A92DD9F96C85E3CDF` (break `/Game/DynamicObjects/Blueprints/InteractionClass/BaseClass/ClassDefaults/ST_Interactable_Details` (`self.InteractDetails`))))))))

(fn `UserConstructionScript`)