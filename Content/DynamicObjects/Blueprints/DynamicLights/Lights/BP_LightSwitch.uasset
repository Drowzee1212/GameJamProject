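; BP_LightSwitch is an interactable switch that toggles every light sharing a configured actor tag.
; On BeginPlay it gathers those actors' light references, intensities and colors through GetLightRefMessage, then applies the StartLightsOn state by presetting LightOn to its inverse.
; InteractRequest and SetLights share one toggle path that writes Brightness and Color material parameters for emissive on/off, then flips LightOn.
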(event `self.ReceiveBeginPlay`
  ;[1 1 1] Begin play
  ;;[1 1 1] Getting all lights
  (`self.GetRoomLights`)
  ;;[1 1 1] Doing this so when reset is called this is negated
  (if (`self.StartLightsOn?`)
    (set `self.LightOn?` false)
    (else
      (set `self.LightOn?` true)))
  (`self.SetLights`))

(event `/Game/DynamicObjects/Blueprints/InteractionClass/BaseClass/Interface/BP_InteractionInteraface.InteractRequest`
  (params (HitObject :type "PrimitiveComponent Object Reference"))
  ;[1 1 1] Flip emissive light on/off
  ;;[1 1 1] Set brightness param
  (for (_array_element _array_index) (`self.LightsAffected`) :!label _label
    (`MaterialInstanceDynamic.SetScalarParameterValue` _array_element "Brightness" (select `bool` (`self.LightOn?`) :`false` (`|GetArrayItem` (`self.LightIntensity`) _array_index) :!type "Float (single-precision)"))
    (`MaterialInstanceDynamic.SetVectorParameterValue` _array_element "Color" (`KismetMathLibrary.Conv_ColorToLinearColor` (`|GetArrayItem` (`self.Color`) _array_index))))
  ;[1 1 1] Flip variable
  (set `self.LightOn?` (not (`self.LightOn?`))))

(event `SetLights`
  ;[1 1 1] Flip emissive light on/off
  ;;[1 1 1] Set brightness param
  (goto _label))

(fn `GetRoomLights`
  ;[1 1 1] Getting lights with specific tag (this basically makes it so that every switch is looking to turn off certain lights)
  (bind _outactors (`GameplayStatics.GetAllActorsWithTag` (`self.LightWithTag`)))
  (for (_array_element _array_index) _outactors
    (bind (_lightref _lightintensity _color) (message `/Game/DynamicObjects/Blueprints/DynamicLights/Interface/BP_LightsInterface.GetLightRef` _array_element))
    (`KismetArrayLibrary.Array_Set` (`self.LightsAffected`) _array_index _lightref true)
    (`KismetArrayLibrary.Array_Set` (`self.LightIntensity`) _array_index _lightintensity true)
    (`KismetArrayLibrary.Array_Set` (`self.Color`) _array_index _color true))
  ;[1 1 1] Create variable for tracking light active
  (for _array_element_2 (`self.LightsAffected`)
    (bind _returnvalue (`MaterialInstanceDynamic.K2_GetScalarParameterValue` _array_element_2 "Brightness"))
    (if (== _returnvalue 0.0)
      (set `self.LightOn?` false)
      (else
        (set `self.LightOn?` true)))))

(fn `UserConstructionScript`)