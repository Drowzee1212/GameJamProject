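; Base Blueprint for a dynamic light object whose three cube meshes switch between dark and bright on a key press.
; On BeginPlay it enables input from the first player controller and gives each cube a dynamic material instance based on the LightSwitch component's material, storing them in an array.
; The M key drives a FlipFlop that sets the Brightness parameter on all stored materials, turning them off on the first press and on at the next.
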(event `self.ReceiveBeginPlay`
  (`self.EnableInput` (`GameplayStatics.GetPlayerController` 0))
  (for (_array_element _array_index) (`|MakeArray` (`self.Cube1`) (`self.Cube2`) (`self.Cube3`))
    (bind _returnvalue (`PrimitiveComponent.CreateDynamicMaterialInstance` _array_element 0 (`PrimitiveComponent.GetMaterial` (`self.LightSwitch`) 0) "None"))
    (`KismetArrayLibrary.Array_Set` (`self.DynamicMaterials`) _array_index _returnvalue true)))

(event `Key|M`
  (params (Key :type "Key Structure"))
  (:`Pressed`
    (`/Engine/EditorBlueprintResources/StandardMacros.FlipFlop`
      (:`A`
        (for _array_element (`self.DynamicMaterials`)
          (`MaterialInstanceDynamic.SetScalarParameterValue` _array_element "Brightness" 0.0)))
      (:`B`
        (for _array_element_2 (`self.DynamicMaterials`)
          (`MaterialInstanceDynamic.SetScalarParameterValue` _array_element_2 "Brightness" 15.0))))))

(fn `UserConstructionScript`)